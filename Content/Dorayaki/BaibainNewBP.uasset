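; BaibainNewBP is a self-replicating actor in the Dorayaki folder that multiplies exponentially in the level.
; On BeginPlay, a looping timer periodically spawns another BaibainNewBP just above its static mesh with a small random horizontal offset.
; Every copy runs its own timer, so the population doubles each interval.
; A shared counter on BP_ThirdPersonCharacter increments on each attempt and stops spawning past a fixed cap.
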(event Custom|spawn1
  (bind _returnvalue (Actor|GetActorOfClass "/Game/ThirdPerson/Blueprints/BP_ThirdPersonCharacter.BP_ThirdPersonCharacter_C"))
  (bind _output_get (Variables|/Game/ThirdPerson/Blueprints/BP_ThirdPersonCharacter.BP_ThirdPersonCharacter_C|SetBaiinBainSpawnCounter _returnvalue (+ (Variables|/Game/ThirdPerson/Blueprints/BP_ThirdPersonCharacter.BP_ThirdPersonCharacter_C|GetBaiinBainSpawnCounter _returnvalue) 1)))
  (if (<= _output_get 512)
    (Game|SpawnActorfromClass "BaibainNewBP_C" (Math|Transform|MakeTransform (+ (Transformation|GetWorldLocation (Variables|Default|GetStaticMesh)) (Math|Vector|MakeVector (Math|Random|RandomFloatinRange -1e+01 1e+01) (Math|Random|RandomFloatinRange -1e+01 1e+01) 1e+01))) "Undefined" "OverrideRootScale" 0 0) ; Classにスポーンしたいメッシュをセットしたブループリントをセットします
  ))

(event EventBeginPlay
  (Utilities|Time|SetTimerbyEvent (delegate Custom|spawn1) 3.0 true) ; Timeには、何秒間隔でスポーンするかをセットします
)

(event Collision|EventActorBeginOverlap
  (params (OtherActor :type Actor%20Object%20Reference)))

(event EventTick
  (params (DeltaSeconds :type Float%20%28single-precision%29)))

(fn ConstructionScript)